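; Actor component that runs a melee AI enemy's combat actions: sword attacks, blocking, weapon equip and unequip.
; A four-step montage combo advances by AttackIndex while the target stays in range; long-range and spinning attacks use montage notifies for sphere damage traces, chasing and AOE slashes.
; It toggles interruptible and blocking flags on BPC_DamageSystem and signals completion through dispatchers.
; BeginPlay finds its enemy through GetActorOfClass rather than GetOwner.
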(event `Attack1`
  (if (<= (`self.Distance`) 400.0)
    (`/Engine/EditorBlueprintResources/StandardMacros.DoOnce` false :!label _label
      (:`Completed`
        (`KismetSystemLibrary.Delay` 0.1)
        (`KismetArrayLibrary.Array_Clear` (`self.Hit Actor`))
        (`|PlayMontage` (stale `ShortRangeSwordAttack` InSkeletalMeshComponent) "/Game/_MSO_Codebase/Animations/AI/SwordAnimations/DefaultAttack/Attack1_Montage.Attack1_Montage"
          (:`then`
            (set `self.AttackIndex` 1)
            (goto _label :!via `Reset`)))))
    (else
      (`self.OnAttackEnded`)
      (set `/Game/_MSO_Codebase/Blueprints/ActorComponents/AI/BPC_DamageSystem.IsInterruptible` true (`self.DamageSystem`)))))

(event `Attack2`
  (if (<= (`self.Distance`) 400.0)
    (`/Engine/EditorBlueprintResources/StandardMacros.DoOnce` false :!label _label_2
      (:`Completed`
        (`KismetSystemLibrary.Delay` 0.1)
        (`KismetArrayLibrary.Array_Clear` (`self.Hit Actor`))
        (`|PlayMontage` (stale `ShortRangeSwordAttack` InSkeletalMeshComponent) "/Game/_MSO_Codebase/Animations/AI/SwordAnimations/DefaultAttack/Attack2_Montage.Attack2_Montage"
          (:`then`
            (set `self.AttackIndex` 2)
            (goto _label_2 :!via `Reset`)))))
    (else
      (`self.OnAttackEnded`)
      (set `/Game/_MSO_Codebase/Blueprints/ActorComponents/AI/BPC_DamageSystem.IsInterruptible` true (`self.DamageSystem`)))))

(event `self.ReceiveBeginPlay`
  (bind _returnvalue (`GameplayStatics.GetActorOfClass` "/Game/_MSO_Codebase/Blueprints/Characters/Ai/BP_Enemy_Melee.BP_Enemy_Melee_C"))
  (set `self.EnemyMelee` _returnvalue)
  (set `self.DamageSystem` (`Actor.GetComponentByClass` _returnvalue "/Game/_MSO_Codebase/Blueprints/ActorComponents/AI/BPC_DamageSystem.BPC_DamageSystem_C")))

(event `Attack3`
  (if (<= (`self.Distance`) 400.0)
    (`/Engine/EditorBlueprintResources/StandardMacros.DoOnce` false :!label _label_3
      (:`Completed`
        (`KismetSystemLibrary.Delay` 0.1)
        (`KismetArrayLibrary.Array_Clear` (`self.Hit Actor`))
        (`|PlayMontage` (stale `ShortRangeSwordAttack` InSkeletalMeshComponent) "/Game/_MSO_Codebase/Animations/AI/SwordAnimations/DefaultAttack/Kick_Montage.Kick_Montage"
          (:`then`
            (set `self.AttackIndex` 3)
            (goto _label_3 :!via `Reset`)))))
    (else
      (`self.OnAttackEnded`)
      (set `/Game/_MSO_Codebase/Blueprints/ActorComponents/AI/BPC_DamageSystem.IsInterruptible` true (`self.DamageSystem`)))))

(event `ShortRangeSwordAttack`
  (params (InSkeletalMeshComponent :type "SkeletalMeshComponent Object Reference") (AttackTarget :type "Actor Object Reference"))
  (set `self.SaveAttack?` true)
  (switch `int` (`self.AttackIndex`) :!label _label_4
    (:`0`
      (`self.Attack1`))
    (:`1`
      (`self.Attack2`))
    (:`2`
      (`self.Attack3`))
    (:`3`
      (`self.Attack4`)))
  (set `/Game/_MSO_Codebase/Blueprints/ActorComponents/AI/BPC_DamageSystem.IsInterruptible` false (`self.DamageSystem`)))

(event `SwordAttackCombo`
  (if (`self.SaveAttack?`)
    (goto _label_4)
    (else
      (`self.StopCombo`))))

(event `Attack4`
  (if (<= (`self.Distance`) 400.0)
    (`/Engine/EditorBlueprintResources/StandardMacros.DoOnce` false :!label _label_5
      (:`Completed`
        (`KismetSystemLibrary.Delay` 0.1)
        (`KismetArrayLibrary.Array_Clear` (`self.Hit Actor`))
        (`|PlayMontage` (stale `ShortRangeSwordAttack` InSkeletalMeshComponent) "/Game/_MSO_Codebase/Animations/AI/SwordAnimations/DefaultAttack/Attack3_Montage.Attack3_Montage"
          (:`then`
            (set `self.AttackIndex` 4)
            (goto _label_5 :!via `Reset`))
          (:`OnCompleted`
            (`self.OnAttackEnded`)
            (set `/Game/_MSO_Codebase/Blueprints/ActorComponents/AI/BPC_DamageSystem.IsInterruptible` true (`self.DamageSystem`))))))
    (else
      (`self.OnAttackEnded`)
      (set `/Game/_MSO_Codebase/Blueprints/ActorComponents/AI/BPC_DamageSystem.IsInterruptible` true (`self.DamageSystem`)))))

(event `StopCombo`
  (set `self.AttackIndex` 0))

(event `UpdateDistanceToTarget`
  (params (Distance :type "Float (double-precision)"))
  (set `self.Distance` Distance))

(event `LongRangeSwordAttack`
  (params (InSkeletalMeshComponent :type "SkeletalMeshComponent Object Reference") (MontageToPlay :type "AnimMontage Object Reference") (AttackTarget :type "Actor Object Reference"))
  (bind _notifyname (`|PlayMontage` InSkeletalMeshComponent MontageToPlay)
    (:`then`
      (set `/Game/_MSO_Codebase/Blueprints/ActorComponents/AI/BPC_DamageSystem.IsInterruptible` false (`self.DamageSystem`)))
    (:`OnCompleted`
      (`self.OnAttackEnded`)
      (set `/Game/_MSO_Codebase/Blueprints/ActorComponents/AI/BPC_DamageSystem.IsInterruptible` true (`self.DamageSystem`) :!label _label_6))
    (:`OnInterrupted`
      (goto _label_6))
    (:`OnNotifyBegin`
      (switch `name` _notifyname
        (:`Slash`
          (`self.DamageTrace`))))))

(event `ChaseAttackTarget`
  (params (AttackTarget :type "Actor Object Reference") (Pawn :type "Pawn Object Reference"))
  (`|AIMoveTo` Pawn (0.0 0.0 0.0) AttackTarget 200.0
    (:`OnSuccess`
      (`KismetSystemLibrary.Delay` 0.1))))

(event `SpiningSwordAttack`
  (params (InSkeletalMeshComponent :type "SkeletalMeshComponent Object Reference") (MontageToPlay :type "AnimMontage Object Reference") (AttackTarget :type "Actor Object Reference") (Pawn :type "Pawn Object Reference") (Instigator :type "Pawn Object Reference") (`Damage Causer` :type "Actor Object Reference"))
  (bind _notifyname (`|PlayMontage` InSkeletalMeshComponent MontageToPlay)
    (:`then`
      (set `/Game/_MSO_Codebase/Blueprints/ActorComponents/AI/BPC_DamageSystem.IsInterruptible` false (`self.DamageSystem`)))
    (:`OnCompleted`
      (`self.OnAttackEnded`)
      (set `/Game/_MSO_Codebase/Blueprints/ActorComponents/AI/BPC_DamageSystem.IsInterruptible` true (`self.DamageSystem`) :!label _label_7))
    (:`OnInterrupted`
      (goto _label_7))
    (:`OnNotifyBegin`
      (switch `name` _notifyname
        (:`Slash`
          (`self.DamageTrace`))
        (:`Spin`
          (`self.ChaseAttackTarget` AttackTarget Pawn))
        (:`AOESlash`
          (`self.AOE_Slash` (`Actor.K2_GetActorLocation` Pawn) Instigator AttackTarget `Damage Causer`))))))

(event `AOE_Slash`
  (params (`Spawn Transform Location` :type "Vector Structure") (Instigator :type "Pawn Object Reference") (AttackTarget :type "Actor Object Reference") (`Damage Causer` :type "Actor Object Reference"))
  (bind _returnvalue (`|SpawnActorFromClass` "/Game/_MSO_Codebase/Blueprints/AI/Actor/AOE/BP_AOE_Base.BP_AOE_Base_C" (`KismetMathLibrary.MakeTransform` `Spawn Transform Location`) "Undefined" "MultiplyWithRoot" null true true false Instigator))
  (set `/Game/_MSO_Codebase/Blueprints/AI/Actor/AOE/BP_AOE_Base.Radius` 300.0 _returnvalue)
  (add `/Game/_MSO_Codebase/Blueprints/AI/Actor/AOE/BP_AOE_Base.OnAOEOverlapActor` _returnvalue (delegate `AOE_DamageActor`))
  (`/Game/_MSO_Codebase/Blueprints/AI/Actor/AOE/BP_AOE_Base.Trigger` _returnvalue))

(event `AOE_DamageActor`
  (params (Actor :type "Actor Object Reference"))
  (if (== Actor (stale `AOE_Slash` AttackTarget))
    (message `/Game/_MSO_Codebase/Blueprints/Interfaces/BPI_Damagable.TakeDamage` Actor (make `/Game/_MSO_Codebase/Blueprints/Structures/S_DamageInfo` 10.0 "NewEnumerator1" "NewEnumerator1") (stale `AOE_Slash` `Damage Causer`))))

(event `EquipWeapon`
  (params (InSkeletalMeshComponent :type "SkeletalMeshComponent Object Reference") (MontageToPlay :type "AnimMontage Object Reference") (WeaponMesh :type "SceneComponent Object Reference") (CharacterMesh :type "SceneComponent Object Reference"))
  (bind _notifyname (`|PlayMontage` InSkeletalMeshComponent MontageToPlay)
    (:`OnCompleted`
      (`self.OnWeaponEquiped`))
    (:`OnNotifyBegin`
      (switch `name` _notifyname
        (:`Hold Sword`
          (`SceneComponent.K2_AttachToComponent` WeaponMesh CharacterMesh "Hand_r_sword_socket" "SnapToTarget" "SnapToTarget" "SnapToTarget" true)
          (set `self.Is Wielding Weapon?` true))))))

(event `UnequipWeapon`
  (params (InSkeletalMeshComponent :type "SkeletalMeshComponent Object Reference") (MontageToPlay :type "AnimMontage Object Reference") (WeaponMesh :type "SceneComponent Object Reference") (CharacterMesh :type "SceneComponent Object Reference"))
  (bind _notifyname (`|PlayMontage` InSkeletalMeshComponent MontageToPlay)
    (:`OnCompleted`
      (`self.OnWeaponUnequiped`))
    (:`OnNotifyBegin`
      (switch `name` _notifyname
        (:`Drop Sword`
          (`SceneComponent.K2_AttachToComponent` WeaponMesh CharacterMesh "Spine_Sword_Socket" "SnapToTarget" "SnapToTarget" "SnapToTarget" true)
          (set `self.Is Wielding Weapon?` false))))))

(event `DestroyWeapon`
  (params (WeaponMesh :type "ActorComponent Object Reference"))
  (`KismetSystemLibrary.Delay` 5.0)
  (`self.K2_DestroyComponent` WeaponMesh))

(event `StartBlock`
  (params (InSkeletalMeshComponent :type "SkeletalMeshComponent Object Reference") (MontageToPlay :type "AnimMontage Object Reference"))
  (`MovementComponent.StopMovementImmediately` (`Character.CharacterMovement` (`self.EnemyMelee`)))
  (set `/Game/_MSO_Codebase/Blueprints/ActorComponents/AI/BPC_DamageSystem.IsBlocking` true (`self.DamageSystem`))
  (set `self.Blocking State` "NewEnumerator1")
  (`|PlayMontage` InSkeletalMeshComponent MontageToPlay
    (:`OnCompleted`
      (`self.EndBlock` :!label _label_8))
    (:`OnInterrupted`
      (if (`|EnumInequality` (`self.Blocking State`) "NewEnumerator2")
        (goto _label_8)))))

(event `OnBlocked`
  (params (InSkeletalMeshComponent :type "SkeletalMeshComponent Object Reference") (MontageToPlay :type "AnimMontage Object Reference"))
  (set `self.Blocking State` "NewEnumerator2")
  (`|PlayMontage` InSkeletalMeshComponent MontageToPlay
    (:`OnCompleted`
      _)
    (:`OnInterrupted`
      _))
  (`self.EndBlock`))

(event `EndBlock`
  (set `/Game/_MSO_Codebase/Blueprints/ActorComponents/AI/BPC_DamageSystem.IsBlocking` false (`self.DamageSystem`))
  (set `self.Blocking State` "NewEnumerator0")
  (`self.OnBlockEnded`))

(event `SetCombatStyleUnarmed`
  (set `self.CombatStyle` "NewEnumerator0"))

(event `SetCombatStyleSwordAndSheild`
  (set `self.CombatStyle` "NewEnumerator1"))

(fn `CalculateFutureActorLocation`
  (params (Actor :type "Actor Object Reference") (Time :type "Float (double-precision)" :default 1.0))
  (returns (Location :type "Vector Structure"))
  (return (+ (`Actor.K2_GetActorLocation` Actor) (* (* (`Actor.GetVelocity` Actor) (1.0 1.0 0.0)) Time))))

(fn `DamageTrace`
  (bind _returnvalue (`self.GetOwner`))
  (bind (_outactors _returnvalue_2) (`KismetSystemLibrary.SphereOverlapActors` (+ (`Actor.K2_GetActorLocation` _returnvalue) (* (`Actor.GetActorForwardVector` _returnvalue) 100.0)) 150.0 (`|MakeArray` "ObjectTypeQuery3" :!type "EObjectTypeQuery Enum") null (`|MakeArray` _returnvalue)))
  (if _returnvalue_2
    (for _array_element _outactors
      (message `/Game/_MSO_Codebase/Blueprints/Interfaces/BPI_Damagable.TakeDamage` _array_element (make `/Game/_MSO_Codebase/Blueprints/Structures/S_DamageInfo` 20.0) _returnvalue)
      (return))))