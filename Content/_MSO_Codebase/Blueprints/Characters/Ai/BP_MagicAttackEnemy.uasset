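; BP_MagicAttackEnemy is an AI mage enemy character whose active attack is a zero-damage radial ground smash.
; MagicAttack and GroundSmashAttack both route to BPCCommonAttack's GroundSmash, while ShortRangeAttack is empty and a montage-driven projectile spell chain through BPCMageEnemy is left unconnected.
; Health, damage and healing functions delegate to BPCDamageSystem, alongside functions for movement speed and ideal combat range.
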(event `self.ShortRangeAttack`)

(event `/Game/_MSO_Codebase/Blueprints/Interfaces/BPI_EnemyAi.Magic_Attack`
  (params (AttackTarget :type "Actor Object Reference"))
  (`/Game/_MSO_Codebase/Blueprints/ActorComponents/AI/BPC_CommonAttack.GroundSmash` (`self.BPC_CommonAttack`) (make `/Game/_MSO_Codebase/Blueprints/Structures/S_AttackInfo` AttackTarget "/Game/_MSO_Codebase/Animations/AI/Magic/mage-ground-smash_Montage.mage-ground-smash_Montage" (make `/Game/_MSO_Codebase/Blueprints/Structures/S_DamageInfo` 0.0)) (`self.Mesh`) (`self.K2_GetActorLocation`) self self 300.0 :!label _label))

(event `/Game/_MSO_Codebase/Blueprints/Interfaces/BPI_EnemyAi.GroundSmashAttack`
  (params (AttackTarget :type "Actor Object Reference"))
  (goto _label))

(fn `GetCurrentHealth`
  (returns (Health :type "Float (double-precision)"))
  (return (`/Game/_MSO_Codebase/Blueprints/ActorComponents/AI/BPC_DamageSystem.Health` (`self.BPC_DamageSystem`))))

(fn `GetIdealRange`
  (returns (AttackRadius :type "Float (double-precision)") (DefendRadius :type "Float (double-precision)"))
  (return 600.0 600.0))

(fn `GetMaxHealth`
  (returns (MaxHealth :type "Float (double-precision)"))
  (return (`/Game/_MSO_Codebase/Blueprints/ActorComponents/AI/BPC_DamageSystem.MaxHealth` (`self.BPC_DamageSystem`))))

(fn `Heal`
  (params (Amount :type "Float (double-precision)"))
  (returns (NewHealth :type "Float (double-precision)"))
  (bind _newhealth (`/Game/_MSO_Codebase/Blueprints/ActorComponents/AI/BPC_DamageSystem.Heal` (`self.BPC_DamageSystem`) Amount))
  (return _newhealth))

(fn `IsDead`
  (returns (Dead :type Boolean))
  (return (`/Game/_MSO_Codebase/Blueprints/ActorComponents/AI/BPC_DamageSystem.IsDead` (`self.BPC_DamageSystem`))))

(fn `SetMovementSpeed`
  (params (Speed :type "/Game/_MSO_Codebase/Blueprints/Enums/E_MovementSpeed Enum" :default "NewEnumerator0"))
  (returns (SpeedValue :type "Float (double-precision)"))
  (bind _output_get (set `CharacterMovementComponent.MaxWalkSpeed` (select `/Game/_MSO_Codebase/Blueprints/Enums/E_MovementSpeed` Speed :`NewEnumerator1` 200.0 :`NewEnumerator2` 300.0 :`NewEnumerator3` 500.0 :!type "Float (single-precision)") (`self.CharacterMovement`)))
  (return _output_get))

(fn `TakeDamage`
  (params (DamageInfo :type "/Game/_MSO_Codebase/Blueprints/Structures/S_DamageInfo Structure") (`Damage Causer` :type "Actor Object Reference"))
  (returns (WasDamaged :type Boolean))
  (bind _wasdamaged (`/Game/_MSO_Codebase/Blueprints/ActorComponents/AI/BPC_DamageSystem.TakeDamage` (`self.BPC_DamageSystem`) DamageInfo `Damage Causer`))
  (return _wasdamaged))

(fn `UserConstructionScript`
  (`parent.UserConstructionScript`))