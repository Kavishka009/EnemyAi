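; Melee sword enemy AI character that offers default, jump and spinning attacks, blocking, and weapon sheathing.
; It is a thin wrapper that forwards combat events to an attack component, passing its mesh, sword and montages.
; A damage system component handles health, healing and attack tokens, and its death and block events trigger sword destruction and block reactions.
; It also reports fixed attack and defend radii as its ideal range.
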(event `self.ReceiveBeginPlay`
  (`parent.ReceiveBeginPlay`))

(event `/Game/_MSO_Codebase/Blueprints/Interfaces/BPI_EnemyAi.DefaultAttack`
  (params (AttackTarget :type "Actor Object Reference"))
  (`/Game/_MSO_Codebase/Blueprints/ActorComponents/AI/BPC_Attack.ShortRangeSwordAttack` (`self.BPC_Attack`) (`self.Mesh`) AttackTarget))

(event `/Game/_MSO_Codebase/Blueprints/Interfaces/BPI_EnemyAi.JumpAttack`
  (params (AttackTarget :type "Actor Object Reference"))
  (`/Game/_MSO_Codebase/Blueprints/ActorComponents/AI/BPC_Attack.LongRangeSwordAttack` (`self.BPC_Attack`) (`self.Mesh`) "/Game/_MSO_Codebase/Animations/AI/SwordAnimations/Jump_attack/sword-jump-attack_Montage.sword-jump-attack_Montage" AttackTarget))

(event `/Game/_MSO_Codebase/Blueprints/Interfaces/BPI_EnemyAi.EquipWeapon`
  (bind _mesh (`self.Mesh`))
  (`/Game/_MSO_Codebase/Blueprints/ActorComponents/AI/BPC_Attack.EquipWeapon` (`self.BPC_Attack`) _mesh "/Game/_MSO_Codebase/Animations/AI/SwordAnimations/sword-Unsheath_Montage.sword-Unsheath_Montage" (`self.Sword_Mesh`) _mesh))

(event `/Game/_MSO_Codebase/Blueprints/Interfaces/BPI_EnemyAi.UnequipWeapon`
  (bind _mesh (`self.Mesh`))
  (`/Game/_MSO_Codebase/Blueprints/ActorComponents/AI/BPC_Attack.UnequipWeapon` (`self.BPC_Attack`) _mesh "/Game/_MSO_Codebase/Animations/AI/SwordAnimations/sword-sheath_Montage.sword-sheath_Montage" (`self.Sword_Mesh`) _mesh))

(event `self.BPC_DamageSystem.OnDeath`
  (`/Game/_MSO_Codebase/Blueprints/ActorComponents/AI/BPC_Attack.DestroyWeapon` (`self.BPC_Attack`) (`self.Sword_Mesh`)))

(event `/Game/_MSO_Codebase/Blueprints/Interfaces/BPI_EnemyAi.StartBlock`
  ;[1 1 1] Blocking
  (`/Game/_MSO_Codebase/Blueprints/ActorComponents/AI/BPC_Attack.StartBlock` (`self.BPC_Attack`) (`self.Mesh`) "/Game/_MSO_Codebase/Animations/AI/SwordAnimations/sword-block_Montage.sword-block_Montage"))

(event `self.BPC_DamageSystem.OnBlocked`
  (params (CanBeParried :type Boolean) (DamageCauser :type "Actor Object Reference"))
  ;[1 1 1] Blocking
  (`/Game/_MSO_Codebase/Blueprints/ActorComponents/AI/BPC_Attack.OnBlocked` (`self.BPC_Attack`) (`self.Mesh`) "/Game/_MSO_Codebase/Animations/AI/SwordAnimations/sword-block-react_Montage.sword-block-react_Montage"))

(event `/Game/_MSO_Codebase/Blueprints/Interfaces/BPI_Damagable.ReturnAttackToken`
  (params (Amount :type Integer))
  (`/Game/_MSO_Codebase/Blueprints/ActorComponents/AI/BPC_DamageSystem.ReturnAttackToken` (`self.BPC_DamageSystem`) Amount))

(event `/Game/_MSO_Codebase/Blueprints/Interfaces/BPI_EnemyAi.UpdateDistanceToTarget`
  (params (Distance :type "Float (double-precision)"))
  (`/Game/_MSO_Codebase/Blueprints/ActorComponents/AI/BPC_Attack.UpdateDistanceToTarget` (`self.BPC_Attack`) Distance))

(event `/Game/_MSO_Codebase/Blueprints/Interfaces/BPI_EnemyAi.SpiningSwordAttack`
  (params (AttackTarget :type "Actor Object Reference"))
  (`/Game/_MSO_Codebase/Blueprints/ActorComponents/AI/BPC_Attack.SpiningSwordAttack` (`self.BPC_Attack`) (`self.Mesh`) AttackTarget self self self (`self.K2_GetActorLocation`)))

(fn `GetCurrentHealth`
  (returns (Health :type "Float (double-precision)"))
  (return (`/Game/_MSO_Codebase/Blueprints/ActorComponents/AI/BPC_DamageSystem.Health` (`self.BPC_DamageSystem`))))

(fn `GetIdealRange`
  (returns (AttackRadius :type "Float (double-precision)") (DefendRadius :type "Float (double-precision)"))
  (return 200.0 350.0))

(fn `GetMaxHealth`
  (returns (MaxHealth :type "Float (double-precision)"))
  (return (`/Game/_MSO_Codebase/Blueprints/ActorComponents/AI/BPC_DamageSystem.MaxHealth` (`self.BPC_DamageSystem`))))

(fn `Heal`
  (params (Amount :type "Float (double-precision)"))
  (returns (NewHealth :type "Float (double-precision)"))
  (bind _newhealth (`/Game/_MSO_Codebase/Blueprints/ActorComponents/AI/BPC_DamageSystem.Heal` (`self.BPC_DamageSystem`) Amount))
  (return _newhealth))

(fn `IsDead`
  (returns (Dead :type Boolean))
  (return (`/Game/_MSO_Codebase/Blueprints/ActorComponents/AI/BPC_DamageSystem.IsDead` (`self.BPC_DamageSystem`))))

(fn `ReserveAttackToken`
  (params (Amount :type Integer))
  (returns (Success :type Boolean))
  (bind _success (`/Game/_MSO_Codebase/Blueprints/ActorComponents/AI/BPC_DamageSystem.ReserveAttackToken` (`self.BPC_DamageSystem`) Amount))
  (return _success))

(fn `TakeDamage`
  (params (DamageInfo :type "/Game/_MSO_Codebase/Blueprints/Structures/S_DamageInfo Structure") (`Damage Causer` :type "Actor Object Reference"))
  (returns (WasDamaged :type Boolean))
  (bind _wasdamaged (`/Game/_MSO_Codebase/Blueprints/ActorComponents/AI/BPC_DamageSystem.TakeDamage` (`self.BPC_DamageSystem`) DamageInfo `Damage Causer`))
  (return _wasdamaged))

(fn `UserConstructionScript`
  (`parent.UserConstructionScript`))