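; Actor component that gives mage enemies two attacks: a targeted dark-energy projectile and a montage-driven ground smash.
; MagicSpell spawns the projectile, which on impact applies damage, reports it to AI damage sensing and signals attack end.
; GroundSmash makes the owner uninterruptible, spawns an AOE on a montage notify that damages only the attack target, then restores interruptibility when the montage completes or is interrupted.
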(event `self.ReceiveBeginPlay`)

(event `MagicSpell`
  (params (SpawnTransform :type "Transform Structure") (Target :type "Actor Object Reference") (DamageInfo :type "/Game/_MSO_Codebase/Blueprints/Structures/S_DamageInfo Structure"))
  (bind _returnvalue (`|SpawnActorFromClass` "/Game/Projectiles/BP_Projectile_DarkEnergy.BP_Projectile_DarkEnergy_C" SpawnTransform "Undefined" "MultiplyWithRoot" (`self.GetOwner`) 1000.0 0.0 Target false null))
  (add `/Game/Projectiles/BP_Projectile_Base.OnProjectileImpact` _returnvalue (delegate `OnProjectileHit`))
  (`PrimitiveComponent.IgnoreActorWhenMoving` (`/Game/Projectiles/BP_Projectile_Base.BoxCollision` _returnvalue) (`self.GetOwner`) true))

(event `OnProjectileHit`
  (params (OtherActor :type "Actor Object Reference") (Hit :type "HitResult Structure"))
  (bind _returnvalue (`self.GetOwner`))
  (message `/Game/_MSO_Codebase/Blueprints/Interfaces/BPI_Damagable.TakeDamage` OtherActor (stale `MagicSpell` DamageInfo) _returnvalue)
  (`AISense_Damage.ReportDamageEvent` OtherActor _returnvalue (`.Amount_2_64864A0D4320D27C3EA14D8019B5EC9D` (break `/Game/_MSO_Codebase/Blueprints/Structures/S_DamageInfo` (stale `MagicSpell` DamageInfo))) (`Actor.K2_GetActorLocation` (`self.GetOwner`)))
  (`self.OnAttackEnd`))

(event `GroundSmash`
  (params (AttackInfo :type "/Game/_MSO_Codebase/Blueprints/Structures/S_AttackInfo Structure") (InSkeletalMeshComponent :type "SkeletalMeshComponent Object Reference") (`Spawn Transform Location` :type "Vector Structure") (Instigator :type "Pawn Object Reference") (`Damage Causer` :type "Actor Object Reference") (Radius :type "Float (single-precision)"))
  (bind (_attacktarget _montage _damageinfo) (break `/Game/_MSO_Codebase/Blueprints/Structures/S_AttackInfo` AttackInfo))
  (bind _returnvalue (`self.GetOwner`))
  (message `/Game/_MSO_Codebase/Blueprints/Interfaces/BPI_EnemyAi.Attack` (`self.GetOwner`) _attacktarget)
  (bind _notifyname (`|PlayMontage` InSkeletalMeshComponent _montage)
    (:`then`
      (message `/Game/_MSO_Codebase/Blueprints/Interfaces/BPI_Damagable.IsInterruptible` _returnvalue false))
    (:`OnCompleted`
      (`self.OnAttackEnd`)
      (message `/Game/_MSO_Codebase/Blueprints/Interfaces/BPI_Damagable.IsInterruptible` _returnvalue true :!label _label))
    (:`OnInterrupted`
      (goto _label))
    (:`OnNotifyBegin`
      (switch `name` _notifyname
        (:`Smash`
          (`self.M_AOE_Slash` `Spawn Transform Location` Instigator _attacktarget `Damage Causer` _damageinfo Radius))))))

(event `M_AOE_Slash`
  (params (`Spawn Transform Location` :type "Vector Structure") (Instigator :type "Pawn Object Reference") (AttackTarget :type "Actor Object Reference") (`Damage Causer` :type "Actor Object Reference") (DamageInfo :type "/Game/_MSO_Codebase/Blueprints/Structures/S_DamageInfo Structure") (Radius :type "Float (single-precision)"))
  (bind _returnvalue (`|SpawnActorFromClass` "/Game/_MSO_Codebase/Blueprints/AI/Actor/AOE/BP_AOE_Base.BP_AOE_Base_C" (`KismetMathLibrary.MakeTransform` `Spawn Transform Location`) "Undefined" "MultiplyWithRoot" null true true false Instigator))
  (set `/Game/_MSO_Codebase/Blueprints/AI/Actor/AOE/BP_AOE_Base.Radius` Radius _returnvalue)
  (add `/Game/_MSO_Codebase/Blueprints/AI/Actor/AOE/BP_AOE_Base.OnAOEOverlapActor` _returnvalue (delegate `M_AOE_DamageActor`))
  (`/Game/_MSO_Codebase/Blueprints/AI/Actor/AOE/BP_AOE_Base.Trigger` _returnvalue))

(event `M_AOE_DamageActor`
  (params (Actor :type "Actor Object Reference"))
  (if (== Actor (stale `M_AOE_Slash` AttackTarget))
    (message `/Game/_MSO_Codebase/Blueprints/Interfaces/BPI_Damagable.TakeDamage` Actor (stale `M_AOE_Slash` DamageInfo) (stale `M_AOE_Slash` `Damage Causer`))))